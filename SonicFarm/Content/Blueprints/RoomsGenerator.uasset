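; Procedural room generator that builds floors, ceilings and walls as static mesh components in the Construction Script, with BeginPlay and Tick left empty.
; A loop steps by CountOfElements through a direction macro, but fixed switch values always add two tiles along +X, occasionally with a small mesh.
; Floors are mapped by location, so a final pass walls every edge lacking a neighbour.
; Earlier random-expansion attempts remain disconnected.
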(event EventBeginPlay)

(event Collision|EventActorBeginOverlap
  (params (OtherActor :type Actor%20Object%20Reference)))

(event EventTick
  (params (DeltaSeconds :type Float%20%28single-precision%29)))

(fn ConstructionScript
  (bind _newvar_0 (Variables|Default|GetNewVar_0))
  (bind _newvar_0_2 (Variables|Default|GetNewVar_0))
  (bind _newvar_2 (Variables|Default|GetNewVar_2))
  (bind _output_get (Variables|Default|SetSaveCountOfElements (Variables|Default|GetCountOfElements)))
  (bind _returnvalue (AddComponent|AddStaticMeshComponent false (Math|Transform|MakeTransform "0, 0, 0" "0, 0, 0" "4.000000,4.000000,0.100000")))
  (bind _output_get_2 (Variables|Default|SetNewVar_1 _returnvalue))
  (Utilities|Array|Add (Variables|Default|GetArrayOfFloors) _output_get_2)
  (Utilities|Map|Add (Variables|Default|GetArrayOfFloors_0) (Variables|/Script/Engine.SceneComponent|GetRelativeLocation _output_get_2) _output_get_2)
  (Utilities|Array|Add (Variables|Default|GetArrayOfLocation) (Variables|/Script/Engine.SceneComponent|GetRelativeLocation _output_get_2))
  (AddComponent|AddStaticMeshComponent false (Math|Transform|MakeTransform "0,0.000000,400.000000" (Variables|Default|GetRelative%20Transform%20Rotation) "4.000000,4.000000,0.100000"))
  (for _index (range 0 (- _output_get 1))
    (switch int 0
      (:Default
        (Rendering|Debug|DrawDebugSphere (Variables|/Script/Engine.SceneComponent|GetRelativeLocation _output_get_2) 5e+01 12 "(R=0.000000,G=1.000000,B=0.009438,A=1.000000)" 5.0))
      (:0
        (Utilities|NewMacro0 (Variables|/Script/Engine.SceneComponent|GetRelativeLocation _output_get_2) (Variables|/Script/Engine.SceneComponent|GetRelativeLocation _output_get_2) (Variables|/Script/Engine.SceneComponent|GetRelativeLocation _output_get_2) (Variables|/Script/Engine.SceneComponent|GetRelativeLocation _output_get_2) :!label _label
          (:then
            (Variables|Default|Set123 "0,1000.000000, 0")
            (Variables|Default|SetRelative%20Transform%20Rotation "0,90.000000,0.000000"))
          (:then2
            (Variables|Default|Set123 "0.000000,-1000.000000, 0")
            (Variables|Default|SetRelative%20Transform%20Rotation "0,90.000000,0.000000"))
          (:then3
            (Variables|Default|Set123 "1000.000000,0.000000, 0")
            (Variables|Default|SetRelative%20Transform%20Rotation "0, 0, 0"))
          (:then4
            (Variables|Default|Set123 "-1000.000000,0.000000, 0")
            (Variables|Default|SetRelative%20Transform%20Rotation "0, 0, 0")))
        (if true
          (switch int 0
            (:0
              (bind _returnvalue_2 (AddComponent|AddStaticMeshComponent false (Math|Transform|MakeTransform _newvar_0 (Math|Rotator|MakeRotator 0.0 0.0 0.0) "4.000000,4.000000,0.100000")))
              (Utilities|Array|AddUnique (Variables|Default|GetArrayOfFloors) _returnvalue_2)
              (Utilities|Map|Add (Variables|Default|GetArrayOfFloors_0) (Variables|/Script/Engine.SceneComponent|GetRelativeLocation _returnvalue_2) _returnvalue_2)
              (bind _returnvalue_3 (AddComponent|AddStaticMeshComponent false (Math|Transform|MakeTransform _newvar_2 (Math|Rotator|MakeRotator 0.0 0.0 0.0) "4.000000,4.000000,0.100000")))
              (bind _output_get_3 (Variables|Default|SetNewVar_1 _returnvalue_3))
              (Utilities|Array|AddUnique (Variables|Default|GetArrayOfFloors) _output_get_3)
              (Utilities|Map|Add (Variables|Default|GetArrayOfFloors_0) (Variables|/Script/Engine.SceneComponent|GetRelativeLocation _output_get_3) _output_get_3)
              (AddComponent|AddStaticMeshComponent false (Math|Transform|MakeTransform (+ _newvar_0 "0, 0,400.000000") (Math|Rotator|MakeRotator 0.0 0.0 0.0) "4.000000,4.000000,0.100000"))
              (AddComponent|AddStaticMeshComponent false (Math|Transform|MakeTransform (+ _newvar_2 "0, 0,400.000000") (Math|Rotator|MakeRotator 0.0 0.0 0.0) "4.000000,4.000000,0.100000"))
              (Utilities|FlowControl|DoN (Variables|Default|GetN)
                (:Exit
                  (if (Math|Random|RandomBoolwithWeight 0.1)
                    (AddComponent|AddStaticMeshComponent false (Math|Transform|MakeTransform (+ _newvar_2 "0, 0,100.000000") (Math|Rotator|MakeRotator 0.0 0.0 0.0) "0.500000,0.500000,0.500000"))
                    (Math|Integer|DecrementInt (Variables|Default|GetN))))))
            (:1
              (bind _returnvalue_4 (AddComponent|AddStaticMeshComponent false (Math|Transform|MakeTransform _newvar_0_2 (Math|Rotator|MakeRotator 0.0 0.0 0.0) "4.000000,4.000000,0.100000")))
              (bind _output_get_4 (Variables|Default|SetNewVar_1 _returnvalue_4))
              (Utilities|Array|AddUnique (Variables|Default|GetArrayOfFloors) _output_get_4)
              (Utilities|Map|Add (Variables|Default|GetArrayOfFloors_0) (Variables|/Script/Engine.SceneComponent|GetRelativeLocation _output_get_4) _output_get_4)
              (AddComponent|AddStaticMeshComponent false (Math|Transform|MakeTransform (+ _newvar_0_2 "0, 0,400.000000") (Math|Rotator|MakeRotator 0.0 0.0 0.0) "4.000000,4.000000,0.100000"))
              (Utilities|FlowControl|DoN (Variables|Default|GetN)
                (:Exit
                  (if (Math|Random|RandomBoolwithWeight 0.1)
                    (AddComponent|AddStaticMeshComponent false (Math|Transform|MakeTransform (+ _newvar_0_2 "0, 0,100.000000") (Math|Rotator|MakeRotator 0.0 0.0 0.0) "0.500000,0.500000,0.500000"))
                    (Math|Integer|DecrementInt (Variables|Default|GetN)))))))
          (else
            (Rendering|Debug|DrawDebugSphere (Variables|/Script/Engine.SceneComponent|GetRelativeLocation _output_get_2) 5e+01 12 "(R=1.000000,G=0.000000,B=0.018015,A=1.000000)" 5.0))))
      (:1
        (goto _label execute2))
      (:2
        (goto _label execute3))
      (:3
        (goto _label execute4))))
  (bind _values (Utilities|Map|Values (Variables|Default|GetArrayOfFloors_0)))
  (for _array_element _values
    (Utilities|FlowControl|Sequence
      (:then_0
        (if (not (Utilities|Map|Contains (Variables|Default|GetArrayOfFloors_0) (+ (Variables|/Script/Engine.SceneComponent|GetRelativeLocation _array_element) "-1000.000000, 0, 0")))
          (Rendering|Debug|DrawDebugSphere (+ (Variables|/Script/Engine.SceneComponent|GetRelativeLocation _array_element) "-1000.000000, 0, 0") 5e+01 12 "(R=0.000000,G=1.000000,B=0.992422,A=1.000000)" 5.0)
          (Variables|Default|SetRelative%20Transform%20Rotation "0, 0, 0")
          (Variables|Default|Set123 (+ (+ (Variables|/Script/Engine.SceneComponent|GetRelativeLocation _array_element) "-1000.000000, 0, 0") "500.000000,0.000000,-100.000000"))
          (if (Math|Random|RandomBool) :!label _label_2
            (AddComponent|AddStaticMeshComponent false (Math|Transform|MakeTransform (Variables|Default|Get123) (Variables|Default|GetRelative%20Transform%20Rotation) "1.000000,5.000000,1.000000"))
            (else
              (AddComponent|AddStaticMeshComponent false (Math|Transform|MakeTransform (Variables|Default|Get123) (Variables|Default|GetRelative%20Transform%20Rotation) "1.000000,5.000000,1.000000"))))))
      (:then_1
        (if (not (Utilities|Map|Contains (Variables|Default|GetArrayOfFloors_0) (+ (Variables|/Script/Engine.SceneComponent|GetRelativeLocation _array_element) "1000.000000, 0, 0")))
          (Rendering|Debug|DrawDebugSphere (+ (Variables|/Script/Engine.SceneComponent|GetRelativeLocation _array_element) "1000.000000, 0, 0") 5e+01 12 "(R=1.000000,G=0.000000,B=0.018015,A=1.000000)" 5.0)
          (Variables|Default|SetRelative%20Transform%20Rotation "0, 0, 0")
          (Variables|Default|Set123 (+ (+ (Variables|/Script/Engine.SceneComponent|GetRelativeLocation _array_element) "1000.000000, 0, 0") "-500.000000,0.000000,-100.000000"))
          (goto _label_2)))
      (:then_2
        (if (not (Utilities|Map|Contains (Variables|Default|GetArrayOfFloors_0) (+ (Variables|/Script/Engine.SceneComponent|GetRelativeLocation _array_element) "0.000000,1000.000000, 0")))
          (Rendering|Debug|DrawDebugSphere (+ (Variables|/Script/Engine.SceneComponent|GetRelativeLocation _array_element) "0.000000,1000.000000, 0") 5e+01 12 "(R=0.476714,G=0.000000,B=1.000000,A=1.000000)" 5.0)
          (Variables|Default|SetRelative%20Transform%20Rotation "0,90.000000,0.000000")
          (Variables|Default|Set123 (+ (+ (Variables|/Script/Engine.SceneComponent|GetRelativeLocation _array_element) "0.000000,1000.000000, 0") "0.000000,-500.000000,-100.000000"))
          (goto _label_2)))
      (:then_3
        (if (not (Utilities|Map|Contains (Variables|Default|GetArrayOfFloors_0) (+ (Variables|/Script/Engine.SceneComponent|GetRelativeLocation _array_element) "0.000000,-1000.000000, 0")))
          (Rendering|Debug|DrawDebugSphere (+ (Variables|/Script/Engine.SceneComponent|GetRelativeLocation _array_element) "0.000000,-1000.000000, 0") 5e+01 12 "(R=0.575629,G=1.000000,B=0.000000,A=1.000000)" 5.0)
          (Variables|Default|SetRelative%20Transform%20Rotation "0,90.000000, 0")
          (Variables|Default|Set123 (+ (+ (Variables|/Script/Engine.SceneComponent|GetRelativeLocation _array_element) "0.000000,-1000.000000, 0") "0.000000,500.000000,-100.000000"))
          (goto _label_2))))))