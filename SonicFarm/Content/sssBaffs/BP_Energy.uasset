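; BP_Energy is an energy pickup actor that triggers when a ThirdPersonCharacter overlaps its BoxEnergy volume.
; On overlap it activates its EnergyUp component, hides the NSPickup2 visual and activates the character's Energy component.
; After a short delay it destroys itself and switches the character's Energy component off, with no change to any energy value.
; The end-overlap event only casts and does nothing further.
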(event OnComponentBeginOverlap(BoxEnergy)
  (params (OverlappedComponent :type Primitive%20Component%20Object%20Reference) (OtherActor :type Actor%20Object%20Reference) (OtherComp :type Primitive%20Component%20Object%20Reference) (OtherBodyIndex :type Integer) (bFromSweep :type Boolean) (SweepResult :type Hit%20Result%20Structure%20%28by%20ref%29))
  (bind _asthird_person_character (Utilities|Casting|CastToThirdPersonCharacter OtherActor))
  (Variables|Default|SetBPThirdPersonCharacter _asthird_person_character)
  (Components|Activation|Activate (Variables|Default|GetEnergyUp) false)
  (Rendering|SetVisibility (Variables|Default|GetNS_Pickup_2) false false)
  (Components|Activation|Activate (Variables|/Game/ThirdPersonBP/Blueprints/ThirdPersonCharacter.ThirdPersonCharacter_C|GetEnergy (Variables|Default|GetBPThirdPersonCharacter)) false)
  (Utilities|FlowControl|Delay 1.0)
  (Actor|DestroyActor)
  (Components|Activation|SetActive (Variables|/Game/ThirdPersonBP/Blueprints/ThirdPersonCharacter.ThirdPersonCharacter_C|GetEnergy (Variables|Default|GetBPThirdPersonCharacter)) false false))

(event OnComponentEndOverlap(BoxEnergy)
  (params (OverlappedComponent :type Primitive%20Component%20Object%20Reference) (OtherActor :type Actor%20Object%20Reference) (OtherComp :type Primitive%20Component%20Object%20Reference) (OtherBodyIndex :type Integer))
  (Utilities|Casting|CastToThirdPersonCharacter OtherActor))

(fn ConstructionScript)