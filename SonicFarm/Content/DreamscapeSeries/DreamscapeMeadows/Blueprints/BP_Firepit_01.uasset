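; Firepit prop for the Dreamscape Meadows environment, with fire, smoke and two lights, configured by an On flag.
; The construction script shows or hides the fire and lowers the smoke when off, but hides both lights in either state.
; Each tick, ShadowedLight interpolates toward a new random point in a box around its starting height, centred on the local XY origin, creating a wandering flicker motion.
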(event EventBeginPlay
  (Variables|Default|SetInitialLoc (.Location (Math|Transform|BreakTransform (Transformation|GetRelativeTransform (Variables|Default|GetShadowedLight))))))

(event Collision|EventActorBeginOverlap
  (params (OtherActor :type Actor%20Object%20Reference)))

(event EventTick
  (params (DeltaSeconds :type Float%20%28single-precision%29))
  (bind _shadowedlight (Variables|Default|GetShadowedLight))
  (Transformation|SetRelativeLocation _shadowedlight (Math|Interpolation|VInterpTo (Variables|/Script/Engine.SceneComponent|GetRelativeLocation _shadowedlight) (Math|Random|RandomPointinBoundingBox (Math|Vector|MakeVector 0.0 0.0 (.Z (Math|Vector|BreakVector (Variables|Default|GetInitialLoc)))) (Math|Vector|MakeVector 1.5e+02 1.5e+02 4e+01)) DeltaSeconds 1.5) false false))

(fn ConstructionScript
  (if (Variables|Default|GetOn?)
    (Rendering|SetVisibility (Variables|Default|GetShadowedLight) false false)
    (Rendering|SetVisibility (Variables|Default|GetAmbientLight) false false)
    (Rendering|SetVisibility (Variables|Default|GetFire) true false)
    (Transformation|AddRelativeLocation (Variables|Default|GetSmoke) "0, 0, 0" false true)
    (else
      (Rendering|SetVisibility (Variables|Default|GetShadowedLight) false false)
      (Rendering|SetVisibility (Variables|Default|GetAmbientLight) false false)
      (Rendering|SetVisibility (Variables|Default|GetFire) false false)
      (Transformation|AddRelativeLocation (Variables|Default|GetSmoke) "0, 0,-40.000000" false true))))