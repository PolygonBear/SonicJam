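; BP_Garden is a garden actor that spawns pickup plants, either a pumpkin or a carrot.
; Separate SpawnPlantPumpkin and SpawnPlantCarrot events each spawn their pickup item slightly above the garden with a random yaw and a zero Z scale.
; Each event stores the new actor in PlantFromThisGarden.
; Neither event is called within this Blueprint, and it has no active BeginPlay, overlap or Tick logic.
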(event Custom|SpawnPlantCarrot
  ;[1 1 1 1 30] Спавн Морковки
  (bind _returnvalue (Game|SpawnActorfromClass "/Game/garden/BP_PickUpItems_Carrot.BP_PickUpItems_Carrot_C" (Math|Transform|MakeTransform (+ (Transformation|GetActorLocation self) "0, 0,20.000000") (Math|Rotator|MakeRotator 0.0 0.0 (.yaw (Math|Random|RandomRotator false))) "1.000000,1.0,0.0") "Undefined" 0 0))
  (Variables|Default|SetPlantFromThisGarden _returnvalue))

(event Custom|SpawnPlantPumpkin
  ;[1 1 1 1 30] Спавн Тыквы
  (bind _returnvalue (Game|SpawnActorfromClass "/Game/garden/BP_PickUpItems_Pumpkin.BP_PickUpItems_Pumpkin_C" (Math|Transform|MakeTransform (+ (Transformation|GetActorLocation self) "0, 0,20.000000") (Math|Rotator|MakeRotator 0.0 0.0 (.yaw (Math|Random|RandomRotator false))) "1.000000,1.0,0.0") "Undefined" 0 0))
  (Variables|Default|SetPlantFromThisGarden _returnvalue))

(event EventBeginPlay)

(event Collision|EventActorBeginOverlap
  (params (OtherActor :type Actor%20Object%20Reference)))

(event EventTick
  (params (DeltaSeconds :type Float%20%28single-precision%29)))

(fn ConstructionScript)