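; Garden pickup actor that grows from half to full scale and then becomes collectable.
; BeginPlay sets the starting scale and enters the growth step, which re-arms a looping GrowPlant timer at the TimerGrow interval and adds a small uniform scale increment.
; Reaching full scale within a tolerance sets CanCollect, which gates further growth, and zeroes TimerGrow.
; The collection logic itself is not in this graph.
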(event Custom|GrowPlant
  (bind _returnvalue (Transformation|GetActorScale3D))
  (if (not (Variables|Default|GetbCanCollect))
    (Utilities|Time|SetTimerbyEvent (delegate Custom|GrowPlant) (Variables|Default|GetTimerGrow) true)
    (Transformation|SetActorScale3D (+ _returnvalue "0.010000,0.010000,0.010000"))
    (if (Math|Vector|Equal(Vector) _returnvalue "1.000000,1.000000,1.000000" 0.0001)
      (Variables|Default|SetTimerGrow 0.0)
      (Variables|Default|SetbCanCollect true))))

(event EventBeginPlay
  (bind _returnvalue (Transformation|GetActorScale3D))
  (Transformation|SetActorScale3D "0.500000,0.500000,0.500000")
  (Utilities|Time|SetTimerbyEvent (delegate Custom|GrowPlant) (Variables|Default|GetTimerGrow) true)
  (Transformation|SetActorScale3D (+ _returnvalue "0.010000,0.010000,0.010000"))
  (if (Math|Vector|Equal(Vector) _returnvalue "1.000000,1.000000,1.000000" 0.0001)
    (Variables|Default|SetTimerGrow 0.0)
    (Variables|Default|SetbCanCollect true)))

(fn ConstructionScript)